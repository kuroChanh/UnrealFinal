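; Base enemy Blueprint that damages player characters within a sphere range and can act as a boss whose death wins the game.
; Sphere overlaps play attack or idle sounds and maintain a list of ThirdPersonCharacters in range.
; A Tick cooldown timer damages every listed character and sets the IsAttack flag.
; Incoming damage drains HitCount; at zero the enemy is destroyed, with bosses first showing the win screen.
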(event `self.Sphere.OnComponentEndOverlap`
  (params (OverlappedComponent :type "PrimitiveComponent Object Reference") (OtherActor :type "Actor Object Reference") (OtherComp :type "PrimitiveComponent Object Reference") (OtherBodyIndex :type Integer))
  ;[1 1 1] Set enemy within attack range
  (`GameplayStatics.PlaySoundAtLocation` (`self.IdleSound`) (`self.K2_GetActorLocation`))
  (bind _asthird_person_character (cast `/Game/ThirdPersonBP/Blueprints/ThirdPersonCharacter` OtherActor))
  (`KismetArrayLibrary.Array_RemoveItem` (`self.ListCharacter`) _asthird_person_character))

(event `self.Sphere.OnComponentBeginOverlap`
  (params (OverlappedComponent :type "PrimitiveComponent Object Reference") (OtherActor :type "Actor Object Reference") (OtherComp :type "PrimitiveComponent Object Reference") (OtherBodyIndex :type Integer) (bFromSweep :type Boolean) (SweepResult :type "HitResult Structure (by ref)"))
  ;[1 1 1] Set enemy within attack range
  (`GameplayStatics.PlaySoundAtLocation` (`self.AttackSound`) (`self.K2_GetActorLocation`))
  (bind _asthird_person_character (cast `/Game/ThirdPersonBP/Blueprints/ThirdPersonCharacter` OtherActor))
  (`KismetArrayLibrary.Array_Add` (`self.ListCharacter`) _asthird_person_character))

(event `self.ReceiveAnyDamage`
  (params (Damage :type "Float (single-precision)") (DamageType :type "DamageType Object Reference") (InstigatedBy :type "Controller Object Reference") (DamageCauser :type "Actor Object Reference"))
  ;[1 1 1] Take Damage
  (bind _output_get (set `self.hitCount` (- (`self.hitCount`) Damage)))
  (if (<= _output_get 0.0)
    (`self.CheckWin`)
    (`self.K2_DestroyActor`)))

(event `self.ReceiveTick`
  (params (DeltaSeconds :type "Float (single-precision)"))
  (bind _listcharacter (`self.ListCharacter`))
  (bind _output_get (set `self.Counter` (+ (`self.Counter`) DeltaSeconds)))
  (if (> _output_get (`self.CoolDownS`))
    (set `self.Counter` 0.0)
    (if (> (`KismetArrayLibrary.Array_Length` _listcharacter) 0)
      (for _array_element _listcharacter
        (`GameplayStatics.ApplyDamage` _array_element (`self.Damage`)))
      (set `self.isAttack` true)
      (else
        (set `self.isAttack` false)))))

(event `WinEvent`
  (`WidgetLayoutLibrary.RemoveAllWidgets`)
  (bind _returnvalue (`|CreateWidget` "/Game/Custom/Widget/WinScreen.WinScreen_C"))
  (`UserWidget.AddToViewport` _returnvalue 0))

(fn `CheckWin`
  (if (`self.isBoss`)
    (if (<= (`self.hitCount`) 0.0)
      (`self.WinEvent`))))

(fn `UserConstructionScript`)