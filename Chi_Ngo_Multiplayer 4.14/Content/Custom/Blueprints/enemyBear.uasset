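; Bear enemy Blueprint that patrols back and forth along the world Y axis.
; BeginPlay fills in its growl sounds, damage, hit count and cooldown, variables this graph sets but never reads.
; Tick runs the parent's tick, then uses the MoveRight flag to flip rotation and step location without sweep, reversing at fixed Y limits.
; The step is a constant per frame, so patrol speed depends on frame rate.
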(event `self.ReceiveBeginPlay`
  (set `self.AttackSound` "/Game/Custom/Audio/Music/bearAttackGrowl.bearAttackGrowl")
  (set `self.IdleSound` "/Game/Custom/Audio/Music/bearIdleGrowl.bearIdleGrowl")
  (set `self.Damage` 0.025)
  (set `self.hitCount` 10.0)
  (set `self.CoolDownS` 3.0))

(event `self.ReceiveTick`
  (params (DeltaSeconds :type "Float (single-precision)"))
  (bind _returnvalue (`self.K2_GetActorLocation`))
  (bind _y (.y _returnvalue))
  (`parent.ReceiveTick` DeltaSeconds)
  (if (`self.moveRight`)
    (`self.K2_SetActorRotation` (struct))
    (`self.K2_SetActorLocation` (+ _returnvalue (0.0 5.0 0.0)))
    (`/Engine/EditorBlueprintResources/StandardMacros.CompareFloat` _y 1500.0
      (:`>`
        (set `self.moveRight` false)))
    (else
      (`self.K2_SetActorRotation` (struct :`Yaw` 180.0))
      (`self.K2_SetActorLocation` (- _returnvalue (0.0 5.0 0.0)))
      (`/Engine/EditorBlueprintResources/StandardMacros.CompareFloat` _y -1000.0
        (:`<`
          (set `self.moveRight` true))))))

(fn `UserConstructionScript`)